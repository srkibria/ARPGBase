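; Actor component that gives an ARPGBaseCharacter owner a physical-animation hit reaction.
; On BeginPlay it adds a PhysicalAnimationComponent to the owner, binds it to the character's mesh and caches that mesh.
; TogglePhysicalAnim enables physics simulation on bodies below the pelvis, excluding the pelvis itself, and applies HitReactionProfile there.
; Despite its name, the toggle only switches the effect on.
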(event `self.ReceiveBeginPlay`
  (bind _returnvalue (`|AddComponentByClass` (`self.GetOwner`) "/Script/Engine.PhysicalAnimationComponent"))
  (bind _output_get (set `self.Physical Animation Component` _returnvalue))
  (bind _asarpgbase_character (cast `ARPGBaseCharacter` (`self.GetOwner`)))
  (bind _mesh (`Character.Mesh` _asarpgbase_character))
  (`PhysicalAnimationComponent.SetSkeletalMeshComponent` _output_get _mesh)
  (set `self.Mesh` _mesh))

(event `TogglePhysicalAnim`
  (`SkeletalMeshComponent.SetAllBodiesBelowSimulatePhysics` (`self.Mesh`) "pelvis" true false)
  (`PhysicalAnimationComponent.ApplyPhysicalAnimationProfileBelow` (`self.Physical Animation Component`) "pelvis" "HitReactionProfile" true false))