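; BP_Attack_Sweep is a sweep attack Blueprint that damages actors its capsule hits while a sweep is active.
; StartSweep and EndSweep toggle the OnSweep flag that gates the capsule's component hit event.
; Each hit actor is added uniquely to HitActors, so it takes a fixed health loss through HealthChange only once per sweep.
; EndSweep clears that list for the next sweep.
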(event `Start Sweep`
  (set `self.bOnSweep` true))

(event `End Sweep`
  (set `self.bOnSweep` false)
  (`KismetArrayLibrary.Array_Clear` (`self.HitActors`)))

(event `self.Capsule.OnComponentHit`
  (params (HitComponent :type "PrimitiveComponent Object Reference") (OtherActor :type "Actor Object Reference") (OtherComp :type "PrimitiveComponent Object Reference") (NormalImpulse :type "Vector Structure") (Hit :type "HitResult Structure (by ref)"))
  (if (`self.bOnSweep`)
    (bind _returnvalue (`KismetArrayLibrary.Array_AddUnique` (`self.HitActors`) OtherActor))
    (if (not (== _returnvalue -1))
      (`ARPGStandardFunctionLibrary.HealthChange` OtherActor -5.0))))

(fn `UserConstructionScript`)